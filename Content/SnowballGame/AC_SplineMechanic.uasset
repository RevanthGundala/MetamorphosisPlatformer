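; Component that draws the predicted snowball arc for the player while not jumping.
; Each tick it line-traces from the camera center and smoothly interpolates the launch origin and aim toward the hit.
; A projectile-path prediction at SnowballSpeed then rebuilds the player's spline, its meshes and the end-sphere marker.
; The slope-based CanJump check is unfinished and never called, and launch speed is still snowball-specific.
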(event EventTick
  (params (DeltaSeconds :type Float%20%28single-precision%29))
  (bind _playerref (Variables|Default|GetPlayerRef))
  (bind _playerref_2 (Variables|Default|GetPlayerRef))
  (bind _spline (Variables|/Game/SnowballGame/BP_PlayerSnow.BP_PlayerSnow_C|GetSpline _playerref_2))
  (bind _spline_2 (Variables|/Game/SnowballGame/BP_PlayerSnow.BP_PlayerSnow_C|GetSpline _playerref))
  ;[1 1 1] Check if our player reference has been set
  (bind _playerref_3 (Variables|Default|GetPlayerRef)
    (:then
      (if (not (Variables|/Game/SnowballGame/BP_PlayerSnow.BP_PlayerSnow_C|GetIsJumping _playerref_3))
        (CallFunction|GetTrace)
        (Default|ClearSplines _playerref_3)
        (bind _predictresult (Class|GameplayStatics|BlueprintPredictProjectilePathAdvanced (Utilities|Struct|MakePredictProjectilePathParams (Variables|Spline|GetSpawnLocation) (* (Math|Vector|GetForwardVector (Variables|Spline|GetSpawnRotation)) (Variables|/Game/SnowballGame/BP_PlayerSnow.BP_PlayerSnow_C|GetSnowballSpeed (Variables|Default|GetPlayerRef))) true 5.0 5.0 true "ECC_Visibility" "ObjectTypeQuery1" (Utilities|Array|MakeArray (Game|Player|GetPlayerPawn 0)))))
        (for _array_element (.PathData (Utilities|Struct|BreakPredictProjectilePathResult _predictresult))
          (Spline|AddSplinePoint _spline (.Location (Utilities|Struct|BreakPredictProjectilePathPointData _array_element)) "Local" true)
          (Transformation|SetWorldLocation (Variables|/Game/SnowballGame/BP_PlayerSnow.BP_PlayerSnow_C|GetSplineEndSphere (Variables|Default|GetPlayerRef)) (Variables|Spline|GetSplineEndLocation) false false))
        (Spline|SetSplinePointType _spline (Utilities|Array|LastIndex (.PathData (Utilities|Struct|BreakPredictProjectilePathResult _predictresult))) "CurveClamped" true)
        (Variables|Spline|SetSplineEndLocation (.Location (Utilities|Struct|BreakPredictProjectilePathPointData (Utilities|Array|Get(acopy) (.PathData (Utilities|Struct|BreakPredictProjectilePathResult _predictresult)) (Utilities|Array|LastIndex (.PathData (Utilities|Struct|BreakPredictProjectilePathResult _predictresult)))))))
        ;[0.1198 0.1198 0.1198] Set tangents for each spline point
        (for _index (range 0 (- (Spline|GetNumberOfSplinePoints _spline_2) 2))
          (Default|SetSplineMeshes (Variables|Default|GetPlayerRef) (.Location (Spline|GetLocationandTangentatSplinePoint _spline_2 _index "Local")) (.Tangent (Spline|GetLocationandTangentatSplinePoint _spline_2 _index "Local")) (.Location (Spline|GetLocationandTangentatSplinePoint _spline_2 (+ _index 1) "Local")) (.Tangent (Spline|GetLocationandTangentatSplinePoint _spline_2 (+ _index 1) "Local"))))))
    (:else
      (Development|PrintString "Player Ref not valid"))))

(fn GetStartandEndTrace
  (bind _returnvalue (Game|GetPlayerCameraManager 0))
  (bind _returnvalue_2 (Transformation|GetActorLocation _returnvalue))
  ;[1 1 1] Trace Start
  (Variables|LineTrace|SetWorldCrosshairLocation _returnvalue_2)
  ;[1 1 1] Trace End
  (Variables|LineTrace|SetImpactPoint (+ _returnvalue_2 (* (Transformation|GetActorForwardVector _returnvalue) 15000))))

(fn GetTraceTransform
  (bind _outhit (Collision|LineTraceByChannel (Variables|LineTrace|GetWorldCrosshairLocation) (Variables|LineTrace|GetImpactPoint) "TraceTypeQuery1" false (Utilities|Array|MakeArray (Game|Player|GetPlayerPawn 0)) "None"))
  (if (.bBlockingHit (Collision|BreakHitResult _outhit))
    (Variables|LineTrace|SetImpactPoint (.ImpactPoint (Collision|BreakHitResult _outhit)))
    (Variables|LineTrace|SetImpactNormal (.ImpactNormal (Collision|BreakHitResult _outhit)))
    (Variables|Spline|SetTargetSpawnLocation (Transformation|GetActorLocation (Game|Player|GetPlayerPawn 0)))
    (Variables|Spline|SetTargetSpawnRotation (Math|Rotator|MakeRotfromX (- (Variables|LineTrace|GetImpactPoint) (Variables|Spline|GetTargetSpawnLocation))))
    (else
      (Development|PrintString "Line Trace did not hit"))))

(fn GetTrace
  (bind _returnvalue (Utilities|Time|GetWorldDeltaSeconds))
  (bind _interpspeed (Variables|Default|GetInterpSpeed))
  (CallFunction|GetStartandEndTrace)
  (CallFunction|GetTraceTransform)
  (Variables|Spline|SetSpawnLocation (Math|Interpolation|VInterpTo (Variables|Spline|GetSpawnLocation) (Variables|Spline|GetTargetSpawnLocation) _returnvalue _interpspeed))
  (Variables|Spline|SetSpawnRotation (Math|Interpolation|RInterpTo (Variables|Spline|GetSpawnRotation) (Variables|Spline|GetTargetSpawnRotation) _returnvalue _interpspeed)))

(fn UpdateCanJump
  ;[1 0.2552 0.2552] TODO: Add more conditions?
  (Variables|Default|SetCanJump (and (< (Class|KismetMathLibrary|DegAcos (Math|Vector|DotProduct (Math|Vector|Normalize (+ (Math|Vector|GetForwardVector (Variables|Spline|GetTargetSpawnRotation)) "0.000000,0.000000,1.000000")) (Math|Vector|Normalize (Variables|LineTrace|GetImpactNormal)))) 7e+01) (not (Variables|/Game/SnowballGame/BP_PlayerSnow.BP_PlayerSnow_C|GetIsJumping (Variables|Default|GetPlayerRef))))))