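; HUD_Meta is the HUD Blueprint that shows the player's health and the game over screen.
; On BeginPlay it adds a W_HUD widget to the viewport and binds UpdateHUD to BP_Player's OnTakeDamage dispatcher.
; UpdateHUD passes new health to the widget's LoseHealth and calls GameOver at zero.
; GameOver adds W_GameOver and pauses the game, leaving its Won input unused.
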(event Custom|Game%20Over
  (params (Won :type Boolean))
  (bind _returnvalue (UserInterface|CreateWidget "/Game/_Core_/Blueprints/UI/W_GameOver.W_GameOver_C" (Game|Player|GetOwningPlayerController)))
  (UserInterface|Viewport|AddtoViewport _returnvalue 0)
  (Game|SetGamePaused true))

(event Custom|Update%20HUD
  (params (NewHealth :type Integer))
  (Default|LoseHealth (Variables|Default|GetHUDWidget) NewHealth)
  (if (== NewHealth 0)
    (CallFunction|GameOver false)))

(event EventBeginPlay
  (bind _returnvalue (UserInterface|CreateWidget "/Game/_Core_/Blueprints/UI/W_HUD.W_HUD_C" (Game|Player|GetOwningPlayerController)))
  (bind _output_get (Variables|Default|SetHUDWidget _returnvalue))
  (UserInterface|Viewport|AddtoViewport _output_get 0)
  (bind _asbp_player (Utilities|Casting|CastToBP_Player (Game|GetPlayerCharacter 0)))
  (bind _output_get_2 (Variables|Default|SetAs%20BP%20Player _asbp_player))
  (EventDispatchers|AssignOnTakeDamage _output_get_2 (delegate Custom|Update%20HUD)))

(fn ConstructionScript)