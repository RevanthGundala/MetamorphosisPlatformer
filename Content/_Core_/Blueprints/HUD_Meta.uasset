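; HUD Blueprint that shows the player's health display and handles the game over screen.
; On BeginPlay it adds a W_HUD widget to the viewport and binds to the OnTakeDamage dispatcher of BP_Player.
; Each damage event passes the new health to the widget's LoseHealth.
; When health equals zero, it adds the W_GameOver widget and pauses the game.
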(event Custom|Game%20Over
  (bind _returnvalue (UserInterface|CreateWidget "/Game/_Core_/UI/W_GameOver.W_GameOver_C" (Game|Player|GetOwningPlayerController)))
  (UserInterface|Viewport|AddtoViewport _returnvalue 0)
  (Game|SetGamePaused true))

(event Custom|Update%20Health%20Widget
  (params (NewHealth :type Integer))
  (Default|LoseHealth (Variables|Default|GetHealthWidget) NewHealth)
  (if (== NewHealth 0)
    (CallFunction|GameOver)))

(event EventBeginPlay
  (bind _returnvalue (UserInterface|CreateWidget "/Game/_Core_/UI/W_HUD.W_HUD_C" (Game|Player|GetOwningPlayerController)))
  (bind _output_get (Variables|Default|SetHealthWidget _returnvalue))
  (UserInterface|Viewport|AddtoViewport _output_get 0)
  (bind _asbp_player (Utilities|Casting|CastToBP_Player (Game|GetPlayerCharacter 0)))
  (bind _output_get_2 (Variables|Default|SetAs%20BP%20Player _asbp_player))
  (EventDispatchers|AssignOnTakeDamage _output_get_2 (delegate Custom|Update%20Health%20Widget)))

(fn ConstructionScript)