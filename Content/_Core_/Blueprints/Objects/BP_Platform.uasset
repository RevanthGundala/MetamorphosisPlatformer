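; BP_Platform is a platform actor with an InterpToMovement component that moves it along configurable control points.
; The construction script applies MoverMesh to the Platform mesh and copies the ControlPoints variable into the movement component.
; For every control point after the first, it adds a copy of the mesh with a transparent material at that position, visualizing the path stops.
; The event graph holds no active logic.
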(event EventBeginPlay)

(event Collision|EventActorBeginOverlap
  (params (OtherActor :type Actor%20Object%20Reference)))

(event EventTick
  (params (DeltaSeconds :type Float%20%28single-precision%29)))

(fn ConstructionScript
  (Components|StaticMesh|SetStaticMesh (Variables|Default|GetPlatform) (Variables|Default|GetMoverMesh))
  (bind _output_get (Variables|/Script/Engine.InterpToMovementComponent|SetControlPoints (Variables|Default|GetInterpToMovement) (Variables|Default|GetControlPoints)))
  (for (_array_element _array_index) _output_get
    (if (!= _array_index 0)
      (bind _returnvalue (AddComponent|AddStaticMeshComponent false (Math|Transform|MakeTransform (.positioncontrolpoint _array_element) "0, 0, 0" "1.000000,1.000000,1.000000")))
      (Components|StaticMesh|SetStaticMesh _returnvalue (Variables|Default|GetMoverMesh))
      (Rendering|Material|SetMaterial _returnvalue 0 "/MeshModelingToolsetExp/Materials/SimpleTwoSidedOffsetMaterial_Transparent.SimpleTwoSidedOffsetMaterial_Transparent"))))