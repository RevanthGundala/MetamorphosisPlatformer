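; Platform actor that responds to the player's jumps through a RotatingMovement component, apparently meant to flip it.
; BeginPlay finds BP_Player and binds RotatePlatform to its OnJump dispatcher.
; A FlipFlop acts only on alternate jumps, activating the movement and immediately deactivating it; the B output is unwired.
; The construction script sets the platform mesh; disconnected leftover code would spawn transparent meshes at control points.
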(event Custom|Rotate%20Platform
  (bind _rotatingmovement (Variables|Default|GetRotatingMovement))
  (Utilities|FlowControl|FlipFlop
    (:A
      (Components|Activation|Activate _rotatingmovement false)
      (Components|Activation|Deactivate _rotatingmovement))))

(event EventBeginPlay
  (bind _returnvalue (Actor|GetActorOfClass "/Game/_Core_/Blueprints/Player/BP_Player.BP_Player_C"))
  (EventDispatchers|AssignOnJump _returnvalue (delegate Custom|Rotate%20Platform)))

(fn ConstructionScript
  (Components|StaticMesh|SetStaticMesh (Variables|Default|GetPlatform) (Variables|Default|GetMoverMesh)))