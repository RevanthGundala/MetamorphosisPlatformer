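; Camera manager actor for a side-scroller that smoothly follows the player.
; Each tick, UpdateCameraPos uses VInterpTo to move the actor toward the player's location plus a look-ahead offset along the player's forward vector.
; The offset's Y is zeroed to prevent zooming in and out.
; LockHeight selects the player's Z when true, otherwise the actor's current Z.
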(event EventTick
  (params (DeltaSeconds :type Float%20%28single-precision%29))
  (CallFunction|UpdateCameraPos))

(fn ConstructionScript)

(fn UpdateCameraPos
  (bind _returnvalue (Transformation|GetActorLocation))
  (bind _player_ref (Variables|Default|GetPlayer%20Ref))
  (bind _camoffset (Variables|Default|GetCamOffset))
  (bind _returnvalue_2 (Transformation|GetActorForwardVector _player_ref))
  (bind _returnvalue_3 (Transformation|GetActorLocation _player_ref))
  (bind _returnvalue_4 (* _returnvalue_2 _camoffset))
  ;[0.04897 0.15 0.01432 0.5] This class deals with side scroller camera
  (Transformation|SetActorLocation (Math|Interpolation|VInterpTo _returnvalue (+ (Math|Vector|MakeVector (.x _returnvalue_3) (.y _returnvalue_3) (Math|Float|SelectFloat (.z _returnvalue_3) (.Z (Math|Vector|BreakVector _returnvalue)) (Variables|Default|GetLockHeight))) (Math|Vector|MakeVector (.x _returnvalue_4) 0.0 (.z _returnvalue_4))) (Utilities|Time|GetWorldDeltaSeconds) (Variables|Default|GetInterp%20Speed)) false false))