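; BP_PatrolRoute is a patrol route that uses a Spline to define a path of points and tracks the current patrol index.
; GoNextPoint steps the index by the patrol direction, reversing it at the last and first points so the route runs back and forth instead of looping.
; GetSplinePointAtWorldPosition returns the world-space location of the spline point at the current index.
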(event Custom|Go%20Next%20Point
  (bind _output_get (Variables|Default|SetPatrolIndex (+ (Variables|Default|GetPatrolIndex) (Variables|Default|GetPatrolDirection))))
  (if (== _output_get (- (Spline|GetNumberOfSplinePoints (Variables|Default|GetSpline)) 1))
    (Variables|Default|SetPatrolDirection -1)
    (elif (== (Variables|Default|GetPatrolIndex) 0)
      (Variables|Default|SetPatrolDirection 1))))

(fn ConstructionScript)

(fn GetSplinePointatWorldPosition
  (return (Spline|GetLocationatSplinePoint (Variables|Default|GetSpline) (Variables|Default|GetPatrolIndex) "World")))